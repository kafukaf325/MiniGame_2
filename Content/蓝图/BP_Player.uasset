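; Player character for a top-down sprite survival game, handling intro animation, movement, health, experience and game-over or results screens.
; Ranged attacks fire pooled bullets toward the cursor when enemies are nearby, and a DataTable row names a looping skill timer.
; Leveling raises attack, upgrades the knife, periodically opens an upgrade menu and unlocks a kill-count burst.
; Hits flash red and grant brief invulnerability by switching collision response.
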(event `开场动画`
  ; 入场动画
  (`KismetSystemLibrary.Delay` 0.2)
  (bind _asabp_player (cast `/Game/蓝图/ABP_Player` (`PaperZDAnimationComponent.AnimInstance` (`self.AnimationComponent`))))
  (set `/Game/蓝图/ABP_Player.isOpening` true _asabp_player)
  (`KismetSystemLibrary.Delay` 0.5)
  (`SceneComponent.SetVisibility` (`self.Sprite`) false false)
  (`SceneComponent.SetVisibility` (`self.sprite-sheet`) true false)
  (`KismetSystemLibrary.Delay` 1.5)
  (`SceneComponent.SetVisibility` (`self.sprite-sheet`) false false)
  (`SceneComponent.SetVisibility` (`self.Sprite`) true false)
  (bind _asabp_player_2 (cast `/Game/蓝图/ABP_Player` (`PaperZDAnimationComponent.AnimInstance` (`self.AnimationComponent`))))
  (set `/Game/蓝图/ABP_Player.isOpening` false _asabp_player_2)
  (`KismetSystemLibrary.PrintString` "解锁"))

(event `self.ReceiveBeginPlay`
  (bind `_as游戏实例` (`/Game/蓝图/实例/公用蓝图函数库.Get游戏实例`))
  ; 初始化
  (`self.开场动画`)
  (set `/Game/蓝图/实例/游戏实例.玩家` self `_as游戏实例`)
  (set `self.As游戏实例` `_as游戏实例`)
  (`self.HUD初始化`)
  (bind _returnvalue (`|GetDataTableRow` "/Game/数据资产/技能数据/技能数据表.技能数据表" "cjb")
    (:`then`
      (bind (_tag `_名字` `_描述` `_释放频率`) (break `/Game/数据资产/技能数据/技能结构` _returnvalue))
      (`KismetSystemLibrary.K2_SetTimer` null _tag `_释放频率` true)
      (bind _returnvalue_2 (`|SpawnActorFromClass` "/Game/技能/BP_技能_2.BP_技能_2_C" (`KismetMathLibrary.MakeTransform` (-10000.0 -10000.0 1000.0)) "Undefined" "MultiplyWithRoot" null null))
      (set `self.技能实例` _returnvalue_2))))

(event `EnhancedInput|/Game/增强输入/IA_Move`
  (params (ActionValue :type "Vector2D Structure") (ElapsedSeconds :type "Float (double-precision)") (TriggeredSeconds :type "Float (double-precision)") (InputAction :type "InputAction Object Reference" :default "/Game/增强输入/IA_Move.IA_Move"))
  (bind (_x _y) (`KismetMathLibrary.BreakVector2D` ActionValue))
  ; 移动
  (:`Triggered`
    (set `self.X` _x)
    (set `self.Y` _y)
    (`self.AddMovementInput` (1.0 0.0 0.0) (`self.X`))
    (`self.AddMovementInput` (0.0 1.0 0.0) (`self.Y`))))

(event `恢复攻击距离`
  ; 10级强化攻击结束
  (set `self.子弹生命周期` (`self.子弹默认生命周期`))
  (set `self.发射子弹动画` "/Game/VFX/NS/Knife/BloodKnife_Lv3.BloodKnife_Lv3"))

(event `/Game/接口/玩家接口.增加经验值`
  (params (`获得经验值` :type "Float (double-precision)"))
  ; 升级
  (bind _output_get (set `self.当前经验值` (+ (`self.当前经验值`) `获得经验值`)))
  (if (>= _output_get (`self.升级经验值`))
    (if (>= (`self.等级`) 10)
      (`self.游戏结算`)
      (else
        (`self.升级`)
        (`self.更新exp界面` :!label _label)))
    (else
      (goto _label))))

(event `/Game/接口/玩家接口.受击`
  (params (`受到伤害` :type "Float (double-precision)") (`攻击者` :type "Actor Object Reference"))
  ; 受击
  (`self.玩家受击HP变化` `受到伤害`)
  (`self.受击闪光`)
  (if (<= (`self.HP`) 0.0)
    (set `self.死亡` true)
    (`GameplayStatics.SetGamePaused` true)
    (bind _returnvalue (`|CreateWidget` "/Game/UI/UI_Gameover.UI_Gameover_C"))
    (bind _output_get (set `self.UI_Gameover` _returnvalue))
    (`UserWidget.AddToViewport` _output_get 0)
    (else
      (`KismetSystemLibrary.K2_SetTimer` null "受击保护" 1.0)
      (`PrimitiveComponent.SetCollisionResponseToChannel` (`self.CapsuleComponent`) "ECC_GameTraceChannel1" "ECR_Ignore")
      (`self.更新HP界面`))))

(event `受击闪光`
  ; 受击
  (`PaperFlipbookComponent.SetSpriteColor` (`self.Sprite`) (struct :`R` 1.0 :`A` 1.0))
  (`KismetSystemLibrary.Delay` 0.2)
  (`PaperFlipbookComponent.SetSpriteColor` (`self.Sprite`) (struct :`R` 1.0 :`G` 1.0 :`B` 1.0 :`A` 1.0)))

(fn `10级强化技能`
  (if (`self.是否强化10级`)
    (bind _output_get (set `self.强化_击杀数量` (+ (`self.强化_击杀数量`) 1)))
    (if (>= _output_get 15)
      (set `self.子弹默认生命周期` (`self.子弹生命周期`))
      (set `self.子弹生命周期` 12.0)
      (set `self.强化_击杀数量` 0)
      (set `self.发射子弹动画` "/Game/VFX/NS/Knife/BloodKnife_LvFinal.BloodKnife_LvFinal")
      (`KismetSystemLibrary.K2_SetTimer` null "恢复攻击距离" 3.0))))

(fn `HUD初始化`
  (bind _returnvalue (`|CreateWidget` "/Game/UI/UI_状态.UI_状态_C"))
  (bind _output_get (set `self.UI_状态` _returnvalue))
  (`UserWidget.AddToViewport` _output_get 0)
  (`self.更新exp界面`)
  (`self.更新HP界面`))

(fn `UserConstructionScript`)

(fn `击杀数量统计`
  (set `self.当前击杀数量` (+ (`self.当前击杀数量`) 1)))

(fn `升级`
  (`ActorComponent.Activate` (`self.Niagara_LevelUp`) true)
  (set `self.等级` (+ (`self.等级`) 1))
  (set `self.当前经验值` (- (`self.当前经验值`) (`self.升级经验值`)))
  (set `self.攻击力` (+ (`self.攻击力`) 10.0))
  (set `self.升级经验值` (+ (`self.升级经验值`) 10.0))
  (`self.武器升级`)
  (`/Game/子弹/对象管理.设置敌人信息` (`/Game/蓝图/实例/游戏实例.对象管理` (`self.As游戏实例`)))
  (if (== (mod (- (`self.等级`) 1) 3) 0)
    (`GameplayStatics.SetGamePaused` true)
    (bind _returnvalue (`|CreateWidget` "/Game/UI/UI_升级.UI_升级_C"))
    (bind _output_get (set `self.UI_升级` _returnvalue))
    (`UserWidget.AddToViewport` _output_get 0)))

(fn `受击保护`
  (`PrimitiveComponent.SetCollisionResponseToChannel` (`self.CapsuleComponent`) "ECC_GameTraceChannel1" "ECR_Overlap"))

(fn `攻击_远程`
  (bind _returnvalue (`self.K2_GetActorLocation`))
  (bind _animinstance (`PaperZDAnimationComponent.AnimInstance` (`self.AnimationComponent`)))
  (bind (_returnvalue_roll _returnvalue_pitch _returnvalue_yaw) (`KismetMathLibrary.BreakRotator` (`KismetMathLibrary.FindLookAtRotation` _returnvalue (`.Location` (`GameplayStatics.BreakHitResult` (`PlayerController.GetHitResultUnderCursorByChannel` (`GameplayStatics.GetPlayerController` 0) "TraceTypeQuery1" true))))))
  (bind (_outactors _returnvalue_2) (`KismetSystemLibrary.SphereOverlapActors` (`self.K2_GetActorLocation`) (* (`CapsuleComponent.GetUnscaledCapsuleRadius` (`self.CapsuleComponent`)) (`self.检测范围`)) (`|MakeArray` "ObjectTypeQuery7" :!type "EObjectTypeQuery Enum") "/Game/敌人/BP_Enemy.BP_Enemy_C"))
  (if _returnvalue_2
    (`/Game/子弹/对象管理.设置子弹池` (`/Game/蓝图/实例/游戏实例.对象管理` (`self.As游戏实例`)) _returnvalue (`self.发射子弹动画`) (`self.攻击力`) (* (`KismetMathLibrary.Conv_RotatorToVector` (`KismetMathLibrary.MakeRotator` 0.0 0.0 _returnvalue_yaw)) 200) (1.0 1.0 1.0) (1.0 1.0 1.0) "Enemy" (`self.子弹生命周期`) 15.0)
    (bind _asabp_player (cast `/Game/蓝图/ABP_Player` _animinstance))
    (set `/Game/蓝图/ABP_Player.isAttacking` true _asabp_player)
    (else
      (bind _asabp_player_2 (cast `/Game/蓝图/ABP_Player` _animinstance))
      (set `/Game/蓝图/ABP_Player.isAttacking` false _asabp_player_2))))

(fn `更新exp界面`
  (`/Game/UI/UI_状态.更新exp` (`self.UI_状态`) (`self.当前经验值`) (`self.升级经验值`))
  (`/Game/UI/UI_状态.更新lv+exp` (`self.UI_状态`) (`self.当前经验值`) (`self.升级经验值`) (`self.等级`)))

(fn `更新HP界面`
  (bind `_aswbp_玩家血条` (cast `/Game/UI/WBP_玩家血条` (`WidgetComponent.GetWidget` (`self.HealthBarWidget`))))
  (`/Game/UI/WBP_玩家血条.设置hp` `_aswbp_玩家血条` (`self.HP`) (`self.最大HP`)))

(fn `检测范围内敌人`)

(fn `武器升级`
  (bind `_等级` (`self.等级`))
  (if (== `_等级` 4)
    (set `self.攻击力` (+ (`self.攻击力`) 10.0))
    (set `self.发射子弹动画` "/Game/VFX/NS/Knife/BloodKnife_Lv2.BloodKnife_Lv2")
    (elif (== `_等级` 7)
      (set `self.子弹生命周期` (* (`self.子弹生命周期`) 1.625))
      (set `self.发射子弹动画` "/Game/VFX/NS/Knife/BloodKnife_Lv3.BloodKnife_Lv3")
      (elif (== `_等级` 10)
        (set `self.是否强化10级` true)))))

(fn `游戏结算`
  (`GameplayStatics.SetGamePaused` true)
  (bind _returnvalue (`|CreateWidget` "/Game/UI/UI_游戏结算.UI_游戏结算_C"))
  (bind _output_get (set `self.UI_游戏结算` _returnvalue))
  (`UserWidget.AddToViewport` _output_get 0))

(fn `玩家受击HP变化`
  (params (`伤害` :type "Float (double-precision)"))
  (set `self.HP` (`KismetMathLibrary.FClamp` (- (`self.HP`) `伤害`) 0.0 (`self.最大HP`)))
  (`self.更新HP界面`))

(fn `获取技能`
  (params (`技能` :type "/Game/UI/Widget/UW_技能 Object Reference"))
  (bind `_技能` (`/Game/UI/Widget/UW_技能.技能` `技能`))
  (`KismetSystemLibrary.PrintString` (`|GetEnumeratorNameAsString` `_技能`))
  (`KismetArrayLibrary.Array_AddUnique` (`self.已学习技能`) `_技能`)
  (set `self.当前持有技能` `_技能`))