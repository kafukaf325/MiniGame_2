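; BP_黑痕 is the Black Scar actor of the electric field skill, a timed damage zone at the field's location.
; 激活黑痕 stores the location and data asset, starts Niagara, runs a one-second looping timer and sets lifespan from the asset.
; 攻击范围敌人 resizes the collision sphere, overlaps for BP_Enemy and calls 受击 with player attack times the configured per-second damage, without knockback.
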(event `攻击范围敌人`
  (bind (`_是否拥有技能` `_每秒造成伤害` `_持续时间` `_范围半径` `_减速百分比` `_是否拥有电荷` `_电荷类型` `_是否可连接其他电场` `_电场连接检测范围` `_最大连接数量` `_电弧额外伤害` `_是否可以爆炸` `_爆炸范围` `_爆炸伤害` `_麻痹范围` `_麻痹减速百分比` `_麻痹持续时间` `_易伤` `_易伤持续时间` `_是否产生黑痕` `_黑痕每秒伤害`) (break `/Game/技能/电场/电场数据配置` (`/Game/技能/电场/电场数据资产.电场数据配置` (`self.电场数据资产`))))
  (`SphereComponent.SetSphereRadius` (`self.SphereCollsion`) `_范围半径` true)
  (bind _outactors (`KismetSystemLibrary.SphereOverlapActors` (`self.黑痕所在位置`) `_范围半径` (`|MakeArray`) "/Game/敌人/BP_Enemy.BP_Enemy_C"))
  (for _array_element _outactors
    (bind _asbp_enemy (cast `/Game/敌人/BP_Enemy` _array_element))
    (bind _asbp_player (cast `/Game/蓝图/BP_Player` (`GameplayStatics.GetPlayerPawn` 0)))
    (`/Game/敌人/BP_Enemy.受击` _asbp_enemy (* (`/Game/蓝图/BP_Player.攻击力` _asbp_player) `_黑痕每秒伤害`) 0.0 false)))

(fn `UserConstructionScript`)

(fn `激活黑痕`
  (params (`电场所在位置` :type "Vector Structure") (`电场数据资产` :type "/Game/技能/电场/电场数据资产 Object Reference"))
  (set `self.黑痕所在位置` `电场所在位置`)
  (bind _output_get (set `self.电场数据资产` `电场数据资产`))
  (`ActorComponent.Activate` (`self.Niagara`) true)
  (bind _returnvalue (`KismetSystemLibrary.K2_SetTimerDelegate` (`|CreateDelegate` :!event `攻击范围敌人`) 1.0 true))
  (set `self.黑痕出伤定时器` _returnvalue)
  (`self.SetLifeSpan` (`.黑痕持续时间_52_D232903540D091FC2759F99C94706ECC` (break `/Game/技能/电场/电场数据配置` (`/Game/技能/电场/电场数据资产.电场数据配置` _output_get)))))