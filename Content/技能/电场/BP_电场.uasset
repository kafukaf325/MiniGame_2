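; BP_电场 is a pooled electric field skill that damages and slows enemies, configured by a data asset.
; 激活电场 starts looping damage and expiry timers; overlap events apply and remove the slow.
; Overlapping fields compare charges: different triggers 过载 explosion damage, same triggers 麻痹 area slow, each once per activation.
; 移除电场 parks the actor off-map, clears timers and decrements the manager's active count.
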(event `攻击范围敌人`
  (bind (`_是否拥有技能` `_每秒造成伤害` `_持续时间` `_范围半径`) (break `/Game/技能/电场/电场数据配置` (`/Game/技能/电场/电场数据资产.电场数据配置` (`self.电场数据资产`))))
  (`SphereComponent.SetSphereRadius` (`self.SphereCollsion`) `_范围半径` true)
  (bind _outactors (`KismetSystemLibrary.SphereOverlapActors` (`self.电场所在位置`) `_范围半径` (`|MakeArray`) "/Game/敌人/BP_Enemy.BP_Enemy_C"))
  (for _array_element _outactors
    (bind _asbp_enemy (cast `/Game/敌人/BP_Enemy` _array_element))
    (bind _asbp_player (cast `/Game/蓝图/BP_Player` (`GameplayStatics.GetPlayerPawn` 0)))
    (`/Game/敌人/BP_Enemy.受击` _asbp_enemy (* (`/Game/蓝图/BP_Player.攻击力` _asbp_player) `_每秒造成伤害`) 0.0 false)))

(event `移除电场`
  (bind `_对象管理` (`/Game/蓝图/实例/游戏实例.对象管理` (`/Game/蓝图/实例/公用蓝图函数库.Get游戏实例`)))
  (`self.K2_SetActorLocation` (10000.0 10000.0 -1000.0))
  (set `self.电场对象状态` "NewEnumerator1")
  (`KismetSystemLibrary.K2_ClearAndInvalidateTimerHandle` (`self.电场回收定时器`))
  (`KismetSystemLibrary.K2_ClearAndInvalidateTimerHandle` (`self.电场出伤定时器`))
  (set `/Game/子弹/对象管理.当前电场数量` (- (`/Game/子弹/对象管理.当前电场数量` `_对象管理`) 1) `_对象管理`)
  (set `self.是否已经过载` false)
  (set `self.是否已经麻痹` false))

(event `self.SphereCollsion.OnComponentBeginOverlap`
  (params (OverlappedComponent :type "PrimitiveComponent Object Reference") (OtherActor :type "Actor Object Reference") (OtherComp :type "PrimitiveComponent Object Reference") (OtherBodyIndex :type Integer) (bFromSweep :type Boolean) (SweepResult :type "HitResult Structure (by ref)"))
  (bind _asbp_enemy (cast `/Game/敌人/BP_Enemy` OtherActor))
  (`/Game/接口/敌人接口.减速` _asbp_enemy (`.减速百分比_8_7FEB2E2E40F5D69B35CFC2B2577DD3FB` (break `/Game/技能/电场/电场数据配置` (`/Game/技能/电场/电场数据资产.电场数据配置` (`self.电场数据资产`))))))

(event `self.SphereCollsion.OnComponentEndOverlap`
  (params (OverlappedComponent :type "PrimitiveComponent Object Reference") (OtherActor :type "Actor Object Reference") (OtherComp :type "PrimitiveComponent Object Reference") (OtherBodyIndex :type Integer))
  (bind _asbp_enemy (cast `/Game/敌人/BP_Enemy` OtherActor))
  (`/Game/接口/敌人接口.取消减速` _asbp_enemy (`.减速百分比_8_7FEB2E2E40F5D69B35CFC2B2577DD3FB` (break `/Game/技能/电场/电场数据配置` (`/Game/技能/电场/电场数据资产.电场数据配置` (`self.电场数据资产`))))))

(event `self.FieldCollsion.OnComponentBeginOverlap`
  (params (OverlappedComponent :type "PrimitiveComponent Object Reference") (OtherActor :type "Actor Object Reference") (OtherComp :type "PrimitiveComponent Object Reference") (OtherBodyIndex :type Integer) (bFromSweep :type Boolean) (SweepResult :type "HitResult Structure (by ref)"))
  (if (`|EnumInequality` (`self.电荷类型`) "NewEnumerator2")
    (if (not (== OtherActor self))
      (bind `_asbp_电场` (cast `/Game/技能/电场/BP_电场` OtherActor))
      (if (`|EnumInequality` (`/Game/技能/电场/BP_电场.电荷类型` `_asbp_电场`) (`self.电荷类型`))
        (`self.过载`)
        (`self.过载` `_asbp_电场`)
        (else
          (`self.麻痹`)
          (`self.麻痹` `_asbp_电场`))))))

(fn `UserConstructionScript`)

(fn `初始化`)

(fn `强化2-2`
  (if (< (`KismetMathLibrary.RandomFloatInRange` 0.0 1.0) 1.0)
    (set `self.电荷类型` "NewEnumerator0")
    (else
      (set `self.电荷类型` "NewEnumerator1"))))

(fn `激活电场`
  (params (`电场数据资产` :type "/Game/技能/电场/电场数据资产 Object Reference") (`电场所在位置` :type "Vector Structure"))
  (set `self.电场对象状态` "NewEnumerator0")
  (set `self.电场所在位置` `电场所在位置`)
  (bind _output_get (set `self.电场数据资产` `电场数据资产`))
  (bind _returnvalue (`KismetSystemLibrary.K2_SetTimerDelegate` (`|CreateDelegate` :!event `攻击范围敌人`) 1.0 true))
  (set `self.电场出伤定时器` _returnvalue)
  (bind _returnvalue_2 (`KismetSystemLibrary.K2_SetTimerDelegate` (`|CreateDelegate` :!event `移除电场`) (`.持续时间_4_7416E4B84561E2C6521934A668DE8672` (break `/Game/技能/电场/电场数据配置` (`/Game/技能/电场/电场数据资产.电场数据配置` _output_get)))))
  (set `self.电场回收定时器` _returnvalue_2)
  (if (`.是否拥有电荷_30_C3A595F14A91BED40FE8FE9F21A46962` (break `/Game/技能/电场/电场数据配置` (`/Game/技能/电场/电场数据资产.电场数据配置` (`self.电场数据资产`))))
    (`self.强化2-2`)))

(fn `过载`
  (bind (`_是否拥有技能` `_每秒造成伤害` `_持续时间` `_范围半径` `_减速百分比` `_是否拥有电荷` `_电荷类型` `_是否可连接其他电场` `_电场连接检测范围` `_最大连接数量` `_电弧额外伤害` `_是否可以爆炸` `_爆炸范围` `_爆炸伤害`) (break `/Game/技能/电场/电场数据配置` (`/Game/技能/电场/电场数据资产.电场数据配置` (`self.电场数据资产`))))
  (if (not (`self.是否已经过载`))
    (set `self.是否已经过载` true)
    (`SphereComponent.SetSphereRadius` (`self.FieldCollsion`) `_爆炸范围` true)
    (bind _outactors (`KismetSystemLibrary.SphereOverlapActors` (`self.电场所在位置`) `_爆炸范围` (`|MakeArray`) "/Game/敌人/BP_Enemy.BP_Enemy_C"))
    (for _array_element _outactors
      (bind _asbp_enemy (cast `/Game/敌人/BP_Enemy` _array_element))
      (bind _asbp_player (cast `/Game/蓝图/BP_Player` (`GameplayStatics.GetPlayerPawn` 0)))
      (`/Game/敌人/BP_Enemy.受击` _asbp_enemy (* (`/Game/蓝图/BP_Player.攻击力` _asbp_player) `_爆炸伤害`) 0.0 false))))

(fn `麻痹`
  (bind (`_是否拥有技能` `_每秒造成伤害` `_持续时间` `_范围半径` `_减速百分比` `_是否拥有电荷` `_电荷类型` `_是否可连接其他电场` `_电场连接检测范围` `_最大连接数量` `_电弧额外伤害` `_是否可以爆炸` `_爆炸范围` `_爆炸伤害` `_麻痹范围` `_麻痹减速百分比`) (break `/Game/技能/电场/电场数据配置` (`/Game/技能/电场/电场数据资产.电场数据配置` (`self.电场数据资产`))))
  (if (not (`self.是否已经麻痹`))
    (set `self.是否已经麻痹` true)
    (`SphereComponent.SetSphereRadius` (`self.FieldCollsion`) `_麻痹范围` true)
    (bind _outactors (`KismetSystemLibrary.SphereOverlapActors` (`self.电场所在位置`) `_麻痹范围` (`|MakeArray`) "/Game/敌人/BP_Enemy.BP_Enemy_C"))
    (for _array_element _outactors
      (bind _asbp_enemy (cast `/Game/敌人/BP_Enemy` _array_element))
      (message `/Game/接口/敌人接口.减速` _asbp_enemy `_麻痹减速百分比`))))