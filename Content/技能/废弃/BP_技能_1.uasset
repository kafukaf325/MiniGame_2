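; Skill Blueprint in the deprecated (废弃) folder, meant to spawn a bonus electric field when a skill triggers.
; Its only function, 附加技能产生, currently just rolls a random float from 0 to 1.
; Disconnected logic switches on BP_Player's held upgrade, tests a per-tier probability, and passes the matching data asset and location to 设置电场池.
; That spawning branch never runs, so no field is produced.
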(fn `附加技能产生`
  (params (`技能产生位置` :type "Vector Structure") (`游戏实例` :type "/Game/蓝图/实例/游戏实例 Object Reference"))
  (set `self.当前生成随机数` (`KismetMathLibrary.RandomFloatInRange` 0.0 1.0)))