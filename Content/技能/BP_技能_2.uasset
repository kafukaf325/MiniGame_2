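; BP_技能_2 is a skill Blueprint that can spawn an electric field as an additional effect at a given position.
; 附加技能产生 reads the player's currently held skill tier and rolls a random chance against that tier's probability.
; On success it selects the matching electric field data asset for that upgrade branch.
; The game instance's object manager then sets up the field through its pool.
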(fn `UserConstructionScript`)

(fn `附加技能产生`
  (params (`技能产生位置` :type "Vector Structure"))
  (bind _returnvalue (< (`self.当前产生随机数`) (`self.强化2_概率`)))
  (bind _returnvalue_2 (< (`self.当前产生随机数`) (`self.强化3_概率`)))
  (set `self.当前产生随机数` (`KismetMathLibrary.RandomFloatInRange` 0.0 1.0))
  (bind _asbp_player (cast `/Game/蓝图/BP_Player` (`GameplayStatics.GetPlayerPawn` 0)))
  (switch `/Game/数据资产/技能数据/E_技能树枚举` (`/Game/蓝图/BP_Player.当前持有技能` _asbp_player)
    (:`NewEnumerator0`
      (if (< (`self.当前产生随机数`) (`self.强化1_概率`))
        (set `self.技能数据资产` "/Game/技能/电场/电场数据资产_强化1.电场数据资产_强化1")
        (`/Game/子弹/对象管理.设置电场池` (`/Game/蓝图/实例/游戏实例.对象管理` (`/Game/蓝图/实例/公用蓝图函数库.Get游戏实例`)) (`local.技能产生位置`) (`self.技能数据资产`) :!label _label)))
    (:`NewEnumerator1`
      (if _returnvalue
        (set `self.技能数据资产` "/Game/技能/电场/电场数据资产_强化2-1.电场数据资产_强化2-1")
        (goto _label)))
    (:`NewEnumerator2`
      (if _returnvalue
        (set `self.技能数据资产` "/Game/技能/电场/电场数据资产_强化2-2.电场数据资产_强化2-2")
        (goto _label)))
    (:`NewEnumerator3`
      (if _returnvalue_2
        (set `self.技能数据资产` "/Game/技能/电场/电场数据资产_强化3-1.电场数据资产_强化3-1")
        (goto _label)))
    (:`NewEnumerator4`
      (if _returnvalue_2
        (set `self.技能数据资产` "/Game/技能/电场/电场数据资产_强化3-2.电场数据资产_强化3-2")
        (goto _label)))))